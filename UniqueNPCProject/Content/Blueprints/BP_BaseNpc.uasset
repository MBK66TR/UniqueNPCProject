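; BP_BaseNpc is a base NPC character that opens an interaction menu and reacts to three options.
; Interact creates WBP_NPCInteraction, hands it a self reference and switches the player to UI-only input with a cursor; HideUI removes the widget without restoring input.
; The option events swap mesh materials, with the third also destroying the NPC after a short delay.
; Tick prints movement velocity for debugging.
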(event `self.Interact`
  (params (Interactor :type "Actor Object Reference"))
  (bind _returnvalue (`|CreateWidget` "/Game/UI/WBP_NPCInteraction.WBP_NPCInteraction_C" (`GameplayStatics.GetPlayerController` 0)))
  (set `self.NewVar` _returnvalue)
  (`/Game/UI/WBP_NPCInteraction.SetNPCReference` _returnvalue self)
  (`UserWidget.AddToViewport` _returnvalue 0)
  (set `PlayerController.bShowMouseCursor` true (`GameplayStatics.GetPlayerController` 0))
  (`WidgetBlueprintLibrary.SetInputMode_UIOnlyEx` (`GameplayStatics.GetPlayerController` 0) null))

(event `self.ExecuteOption1`
  (params (Interactor :type "Actor Object Reference"))
  (`PrimitiveComponent.SetMaterial` (`self.Mesh`) 0 "/Game/StarterContent/Materials/M_Brick_Clay_Beveled.M_Brick_Clay_Beveled"))

(event `self.ExecuteOption2`
  (params (Interactor :type "Actor Object Reference"))
  (`PrimitiveComponent.SetMaterial` (`self.Mesh`) 1 "/Game/StarterContent/Materials/M_CobbleStone_Rough.M_CobbleStone_Rough"))

(event `self.ExecuteOption3`
  (params (Interactor :type "Actor Object Reference"))
  (`PrimitiveComponent.SetMaterial` (`self.Mesh`) 0 "/Game/StarterContent/Props/Materials/M_Lamp.M_Lamp")
  (`KismetSystemLibrary.Delay` 1.0)
  (`self.K2_DestroyActor`))

(event `self.ReceiveTick`
  (params (DeltaSeconds :type "Float (single-precision)"))
  (`KismetSystemLibrary.PrintString` (`KismetStringLibrary.Conv_VectorToString` (`MovementComponent.Velocity` (`self.CharacterMovement`))) true true (struct :`G` 0.66 :`B` 1.0 :`A` 1.0) 0.0))

(fn `HideUI`
  (bind _newvar (`self.NewVar`))
  (`Widget.SetVisibility` _newvar "Hidden")
  (`Widget.RemoveFromParent` _newvar))

(fn `UserConstructionScript`)